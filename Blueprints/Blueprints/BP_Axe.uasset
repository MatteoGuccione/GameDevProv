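; BP_Axe is an axe actor that can be picked up and dropped through Attach and Detach events.
; Attach records the owner and disables collision without attaching any component itself; Detach clears the owner, restores collision and enables mesh physics.
; On Solved, the mesh moves to any location stored under the actor's display name in the GameInstance's NamePositionMessage map.
; IsAttachedOutput always returns false, ignoring the IsAttached flag.
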(event EventBeginPlay
  (|CallParentFunction) ; This node is disabled and will not be called.\nDrag off pins to build functionality.
)

(event Collision|EventActorBeginOverlap
  (params (OtherActor :type Actor%20Object%20Reference))
  (|CallParentFunction OtherActor) ; This node is disabled and will not be called.\nDrag off pins to build functionality.
)

(event EventDetach
  (Variables|Default|SetattachedTo 0)
  (Physics|SetSimulatePhysics (Variables|Default|GetStaticMesh) true)
  (Collision|SetActorEnableCollision self true)
  (Variables|Default|SetIs%20Attached false))

(event EventAttach
  (params (Owner :type Actor%20Object%20Reference))
  (Variables|Default|SetattachedTo Owner)
  (Collision|SetActorEnableCollision self false)
  (Variables|Default|SetIs%20Attached true))

(event EventSolved
  (bind _nameposition (Class|IGet|GetNamePosition(Message) (Game|GetGameInstance)))
  (if (.ReturnValue (Utilities|Map|Find _nameposition (Utilities|GetDisplayName self)))
    (Transformation|SetWorldLocation (Variables|Default|GetStaticMesh) (.Value (Utilities|Map|Find _nameposition (Utilities|GetDisplayName self))) false false)))

(event EventTick
  (params (DeltaSeconds :type Float%20%28single-precision%29)))

(fn ConstructionScript
  (|CallParentFunction))

(fn IsAttachedOutput
  (return false))