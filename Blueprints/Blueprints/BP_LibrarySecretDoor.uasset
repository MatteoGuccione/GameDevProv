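; Library secret door puzzle that opens when the player inserts the correct BP_Tome.
; Interaction attaches the carried tome and shows self-dialogue, offset by a GameInstance counter; a wrong book is ejected on the next interaction.
; The correct book registers the solve through ResolvedBy, triggering a timeline that slides the actor along Y.
; BeginPlay replays the opening if the GameInstance already records the Library puzzle as solved.
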(event EventBeginPlay
  (|CallParentFunction)
  (bind _solvedpuzzles (Class|IGet|GetSolvedPuzzle(Message) (Game|GetGameInstance)))
  (if (Utilities|Set|Contains _solvedpuzzles "Library")
    (CallFunction|Resolve)))

(event Collision|EventActorBeginOverlap
  (params (OtherActor :type Actor%20Object%20Reference))
  (|CallParentFunction OtherActor) ; This node is disabled and will not be called.\nDrag off pins to build functionality.
)

(event EventTick
  (params (DeltaSeconds :type Float%20%28single-precision%29))
  (|CallParentFunction DeltaSeconds))

(event EventResolvedby
  (params (Resolver :type Actor%20Object%20Reference))
  (bind _solvedlibraries (Variables|Default|GetsolvedLibraries))
  (if (not (Utilities|Set|Contains _solvedlibraries Resolver))
    (Utilities|Set|Add _solvedlibraries Resolver)
    (if (== (Utilities|Set|Length _solvedlibraries) 1)
      (CallFunction|Resolve))))

(event EventResolve
  (Variables|Default|Setlocation (Transformation|GetActorLocation))
  (bind _rotate (Timeline|Rotating Play)
    (:Update
      (Transformation|SetActorLocation (Math|Vector|Lerp(Vector) (Variables|Default|Getlocation) (+ (Variables|Default|Getlocation) (Math|Vector|MakeVector 0.0 (Variables|Default|GetMovement) 0.0)) _rotate) false false))))

(event EventInteraction
  (bind _returnvalue (Transformation|GetActorLocation))
  (bind _returnvalue_2 (Game|GetGameInstance))
  (bind _self self)
  (bind _returnvalue_3 (Transformation|GetActorRotation _self))
  (if (not (Variables|Default|GetSolvedBool))
    (if (Utilities|IsValid (Variables|Default|GetreferenceActor))
      (Class|IControlAttach|Detach(Message) (Variables|Default|GetreferenceActor))
      (Transformation|SetActorLocation (Variables|Default|GetreferenceActor) (Math|Vector|MakeVector (+ (.x _returnvalue) (Variables|Default|GetPushTomeX)) (- (.y _returnvalue) 1.2e+02) (+ (.z _returnvalue) 1.2e+02)) false true)
      (Collision|SetActorEnableCollision true)
      (Variables|Default|SetreferenceActor 0)
      (else
        (bind _actor (Class|IGet|GetAttachedActorLocal(Message) _returnvalue_2))
        (if (and (Utilities|IsValid _actor) (== (Utilities|GetClass _actor) "/Game/Custom/Blueprints/Blueprints/BP_Tome.BP_Tome_C"))
          (bind _output_get (Variables|Default|SetreferenceActor _actor))
          (Class|IControlAttach|Detach(Message) _output_get)
          (Class|ISave|SaveAttachedActorLocal(Message) _returnvalue_2)
          (Transformation|AttachActorToActor (Variables|Default|GetreferenceActor) self "None" "SnapToTarget" "SnapToTarget" "KeepWorld" true)
          (Transformation|AddActorLocalOffset (Variables|Default|GetreferenceActor) "25.000000,175.000000,120.000000" false false)
          (Transformation|SetActorRotation (Variables|Default|GetreferenceActor) (Math|Rotator|MakeRotator (.roll _returnvalue_3) (+ (.pitch _returnvalue_3) 9e+01) (.yaw _returnvalue_3)))
          (bind _returnvalue_4 (UserInterface|CreateWidget "/Game/Custom/Blueprints/Widgets/WB_SelfDialogue.WB_SelfDialogue_C" (Game|GetPlayerController 0)))
          (Variables|Default|SetselfDialogueWidget _returnvalue_4)
          (if (== (Variables|Default|GetreferenceActor) (Variables|Default|GetcorrectBook))
            (Variables|/Script/UMG.TextBlock|SetText (Variables|/Game/Custom/Blueprints/Widgets/WB_SelfDialogue.WB_SelfDialogue_C|GetDialogue (Variables|Default|GetselfDialogueWidget)) "This should be it")
            (Collision|SetActorEnableCollision (Variables|Default|GetreferenceActor) false)
            (Class|IDestroy|DestroyAttachedActor(Message) (Game|Player|GetPlayerPawn 0) false)
            (Variables|Default|SetSolvedBool true)
            (CallFunction|Resolvedby self)
            (else
              (Variables|/Script/UMG.TextBlock|SetText (Variables|/Game/Custom/Blueprints/Widgets/WB_SelfDialogue.WB_SelfDialogue_C|GetDialogue (Variables|Default|GetselfDialogueWidget)) "I feel like this is wrong")
              (Collision|SetActorEnableCollision (Variables|Default|GetreferenceActor) false)
              (Class|IDestroy|DestroyAttachedActor(Message) (Game|Player|GetPlayerPawn 0) false)))
          (bind _number (Class|IGet|GetSelfDialogueNumber(Message) (Game|GetGameInstance)))
          (bind _output_get_2 (Variables|Default|SetdialogueNumber _number))
          (UserInterface|Viewport|AddtoViewport (Variables|Default|GetselfDialogueWidget) 0)
          (switch int _output_get_2
            (:Default
              (Development|PrintString "Hello"))
            (:0
              (Class|UserWidget|SetPositioninViewport (Variables|Default|GetselfDialogueWidget) "(X=0.000000,Y=50.000000)" false)
              (Class|ISave|SaveSelfDialogueNumber(Message) (Game|GetGameInstance) (+ 1 (Variables|Default|GetdialogueNumber)) :!label _label)
              (Utilities|FlowControl|Delay 2.0)
              (Widget|RemovefromParent (Variables|Default|GetselfDialogueWidget))
              (Class|ISave|SaveSelfDialogueNumber(Message) (Game|GetGameInstance) (Variables|Default|GetdialogueNumber)))
            (:1
              (Class|UserWidget|SetPositioninViewport (Variables|Default|GetselfDialogueWidget) "(X=0.000000,Y=100.000000)" false)
              (goto _label))
            (:2
              (Class|UserWidget|SetPositioninViewport (Variables|Default|GetselfDialogueWidget) "(X=0.000000,Y=150.000000)" false)
              (goto _label))))))))

(fn ConstructionScript
  (|CallParentFunction))