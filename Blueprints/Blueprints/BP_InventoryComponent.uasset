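; Inventory component that holds a ten-slot item array and shows it in WB_Inventory, toggled with the I key along with mouse cursor and look input.
; GetItem scans slots in order, stacking matching items up to a limit or filling an empty slot, then hides the picked-up actor and disables its collision.
; RemoveItem clears the first name-matched slot.
; Both functions refresh the widget and report changes to the GameInstance through messages.
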(event EventBeginPlay
  (bind _returnvalue (UserInterface|CreateWidget "/Game/Custom/Blueprints/Widgets/Inventory/Widgets/WB_Inventory.WB_Inventory_C"))
  (Variables|Default|SetInventoryWidget _returnvalue)
  (Utilities|Array|Resize (Variables|Default|GetItems) 10)
  (Default|LoadInventory (Variables|Default|GetInventoryWidget) self))

(event EventTick
  (params (DeltaSeconds :type Float%20%28single-precision%29)))

(event Input|KeyboardEvents|I
  (params (Key :type Key%20Structure :default "None"))
  (bind _returnvalue (Game|GetPlayerController 0))
  (bind _inventorywidget (Variables|Default|GetInventoryWidget))
  (:Pressed
    (Utilities|FlowControl|FlipFlop
      (:A
        (UserInterface|Viewport|AddtoViewport _inventorywidget 0)
        (Widget|SetVisibility _inventorywidget "Visible")
        (Variables|/Script/Engine.PlayerController|SetbShowMouseCursor _returnvalue true)
        (Input|SetIgnoreLookInput _returnvalue true))
      (:B
        (Widget|RemovefromParent _inventorywidget)
        (Widget|SetVisibility _inventorywidget "Hidden")
        (Variables|/Script/Engine.PlayerController|SetbShowMouseCursor _returnvalue false)
        (Input|SetIgnoreLookInput _returnvalue false)))))

(fn GetItem
  (params (Item :type Actor%20Object%20Reference))
  (bind _struct (Class|IGet|GetItemStruct(Message) Item))
  (bind (_array_element _array_index) (Utilities|Array|ForEachLoopwithBreak (Variables|Default|GetItems) :!label _label)
    (:LoopBody
      (if (Math|Boolean|ANDBoolean (Utilities|Enum|Equal(Enum) (.Name (Utilities|Struct|BreakS_ItemStructure _array_element)) (.Name (Utilities|Struct|BreakS_ItemStructure _struct))) (.Stackable (Utilities|Struct|BreakS_ItemStructure _struct)) (<= (+ (.Quantity (Utilities|Struct|BreakS_ItemStructure _array_element)) (.Quantity (Utilities|Struct|BreakS_ItemStructure _struct))) 64))
        (Utilities|Array|SetArrayElem (Variables|Default|GetItems) _array_index (Utilities|Struct|MakeS_ItemStructure (.Name (Utilities|Struct|BreakS_ItemStructure _struct)) (.Stackable (Utilities|Struct|BreakS_ItemStructure _struct)) (+ (.Quantity (Utilities|Struct|BreakS_ItemStructure _array_element)) (.Quantity (Utilities|Struct|BreakS_ItemStructure _struct))) (.Image (Utilities|Struct|BreakS_ItemStructure _struct)) (.Mesh (Utilities|Struct|BreakS_ItemStructure _struct)) Item))
        (Default|LoadInventory (Variables|Default|GetInventoryWidget) self :!label _label_2)
        (Class|ISave|SaveIteminInventory(Message) (Game|GetGameInstance) _struct)
        (Rendering|SetActorHiddenInGame Item true)
        (Collision|SetActorEnableCollision Item false)
        (goto _label Break)
        (elif (== (.Quantity (Utilities|Struct|BreakS_ItemStructure _array_element)) 0)
          (Utilities|Array|SetArrayElem (Variables|Default|GetItems) _array_index (Utilities|Struct|MakeS_ItemStructure (.Name (Utilities|Struct|BreakS_ItemStructure _struct)) (.Stackable (Utilities|Struct|BreakS_ItemStructure _struct)) (.Quantity (Utilities|Struct|BreakS_ItemStructure _struct)) (.Image (Utilities|Struct|BreakS_ItemStructure _struct)) (.Mesh (Utilities|Struct|BreakS_ItemStructure _struct)) Item))
          (goto _label_2))))))

(fn RemoveItem
  (params (Actor :type S%20Item%20Structure%20Structure))
  (bind (_array_element _array_index) (Utilities|Array|ForEachLoopwithBreak (Variables|Default|GetItems) :!label _label)
    (:LoopBody
      (if (Utilities|Enum|Equal(Enum) (.Name (Utilities|Struct|BreakS_ItemStructure Actor)) (.name _array_element))
        (Utilities|Array|SetArrayElem :TargetArray (Variables|Default|GetItems) :Index _array_index)
        (Class|IRemove|RemovefromInventory(Message) (Game|GetGameInstance) _array_index)
        (goto _label Break)))
    (:Completed
      (Default|LoadInventory (Variables|Default|GetInventoryWidget) self))))