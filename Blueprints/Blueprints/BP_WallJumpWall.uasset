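; BP_WallJumpWall is a wall actor that tracks whether it is currently available for a wall jump.
; SaveAvailableforWallJump stores the passed availability, then sets it back to true after a short delay, acting as a per-wall cooldown.
; GetIsAvailableForWallJump exposes that flag; the other getters, which look like a shared interface, are stubs returning defaults.
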(event EventBeginPlay)

(event Collision|EventActorBeginOverlap
  (params (OtherActor :type Actor%20Object%20Reference)))

(event EventTick
  (params (DeltaSeconds :type Float%20%28single-precision%29)))

(event EventSaveAvailableforWallJump
  (params (available :type Boolean))
  (Variables|Default|SetavailableWJ available)
  (Utilities|FlowControl|Delay 1.4)
  (Variables|Default|SetavailableWJ true))

(fn ConstructionScript)

(fn GetActortoNotSpawn
  (return false))

(fn GetActorVelocity
  (return "0, 0, 0"))

(fn GetAttachedActor
  (return 0))

(fn GetAttachedActorLocal
  (return 0))

(fn GetAttachedActorName
  (return ""))

(fn GetAvailableJump
  (return 0))

(fn GetFirstStart
  (return false))

(fn Getinventory
  (return 0))

(fn GetIsAvailableforWallJump
  (return (Variables|Default|GetavailableWJ)))

(fn GetItemsinInventory
  (return 0))

(fn GetItemStruct
  (return ""))

(fn GetKeys
  (return 0))

(fn GetNamePosition
  (return 0))

(fn GetPlayer&Actor
  (return 0))

(fn GetPlayerAbleTeleport
  (return false))

(fn GetPlayerForward
  (return "0, 0, 0"))

(fn GetSelfDialogueNumber
  (return 0))

(fn GetSolvedActorLocal
  (return 0))

(fn GetSolvedActors
  (return 0))

(fn GetSolvedPuzzle
  (return 0))