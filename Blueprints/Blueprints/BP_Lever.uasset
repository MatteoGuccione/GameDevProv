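; BP_Lever is a lever actor that removes itself from the level if it is recorded as solved.
; On BeginPlay it runs the parent logic, then gets the solved-actors data from the Game Instance and destroys itself if its own display name is found there.
; Persistence is keyed by display name, and any other behavior comes from the parent class, as the overlap and tick events are inactive.
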(event EventBeginPlay
  (|CallParentFunction)
  (bind _solvedactors (Class|IGet|GetSolvedActors(Message) (Game|GetGameInstance)))
  (if (Utilities|Array|ContainsItem _solvedactors (Utilities|GetDisplayName self))
    (Actor|DestroyActor)))

(event Collision|EventActorBeginOverlap
  (params (OtherActor :type Actor%20Object%20Reference))
  (|CallParentFunction OtherActor) ; This node is disabled and will not be called.\nDrag off pins to build functionality.
)

(event EventTick
  (params (DeltaSeconds :type Float%20%28single-precision%29)))

(fn ConstructionScript
  (|CallParentFunction))