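; BP_Blocked is an actor that moves vertically when the player pawn enters its Box trigger.
; On overlap it stores its current location and plays a Timeline that lerps it along Z to that location minus Movement, without sweeping.
; The graph has no reverse or reset logic, and BeginPlay, Tick and the construction script are empty.
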(event OnComponentBeginOverlap(Box)
  (params (OverlappedComponent :type Primitive%20Component%20Object%20Reference) (OtherActor :type Actor%20Object%20Reference) (OtherComp :type Primitive%20Component%20Object%20Reference) (OtherBodyIndex :type Integer) (bFromSweep :type Boolean) (SweepResult :type Hit%20Result%20Structure%20%28by%20ref%29))
  (if (== OtherActor (Game|Player|GetPlayerPawn 0))
    (Variables|Default|Setlocation (Transformation|GetActorLocation))
    (bind _newtrack_0 (Timeline|Timeline Play)
      (:Update
        (Transformation|SetActorLocation (Math|Vector|Lerp(Vector) (Variables|Default|Getlocation) (- (Variables|Default|Getlocation) (Math|Vector|MakeVector 0.0 0.0 (Variables|Default|GetMovement))) _newtrack_0) false false)))))

(event EventBeginPlay)

(event Collision|EventActorBeginOverlap
  (params (OtherActor :type Actor%20Object%20Reference)))

(event EventTick
  (params (DeltaSeconds :type Float%20%28single-precision%29)))

(fn ConstructionScript)