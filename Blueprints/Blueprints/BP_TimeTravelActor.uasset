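; Time-travel actor that the player can attach and detach, with its position persisted in the Game Instance.
; Attach disables collision and saves the mesh location under the actor's display name; Detach restores collision, enables physics and replaces that entry.
; Solved moves the mesh to any saved location, removes the entry, then reattaches the actor to the player if the Game Instance reports an attachment.
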(event EventIsAttachedInput
  (params (isAttachedInput :type Boolean))
  (Variables|Default|SetisAttached isAttachedInput))

(event Collision|EventActorBeginOverlap
  (params (OtherActor :type Actor%20Object%20Reference)))

(event EventDetach
  (bind _self self)
  (Variables|Default|SetattachedTo 0)
  (Physics|SetSimulatePhysics (Variables|Default|GetStaticMesh) true)
  (Collision|SetActorEnableCollision self true)
  (Variables|Default|SetisAttached false)
  (Class|IRemove|RemoveActor(Message) (Game|GetGameInstance) _self)
  (Class|ISave|SavePositionName(Message) (Game|GetGameInstance) (Utilities|GetDisplayName _self) (Transformation|GetWorldLocation (Variables|Default|GetStaticMesh _self))))

(event EventAttach
  (params (Owner :type Actor%20Object%20Reference))
  (bind _self self)
  (Variables|Default|SetattachedTo Owner)
  (Collision|SetActorEnableCollision self false)
  (Variables|Default|SetisAttached true)
  (Class|ISave|SavePositionName(Message) (Game|GetGameInstance) (Utilities|GetDisplayName _self) (Transformation|GetWorldLocation (Variables|Default|GetStaticMesh _self))))

(event EventSolved
  (bind _returnvalue (Game|GetGameInstance))
  (bind _self self)
  ;[1 1 1] Check if this specific actor, found using his display name, has a position saved. If he has he is moved to that location and than removed from the dict of actor saved
  (bind _nameposition (Class|IGet|GetNamePosition(Message) (Game|GetGameInstance)))
  (if (.ReturnValue (Utilities|Map|Find _nameposition (Utilities|GetDisplayName self)))
    (Transformation|SetWorldLocation (Variables|Default|GetStaticMesh) (.Value (Utilities|Map|Find _nameposition (Utilities|GetDisplayName self))) false false)
    (Class|IRemove|RemoveActor(Message) (Game|GetGameInstance) _self)
    ;[1 1 1] Check if he is supposed to be attached to the player. If he is, he attach himself to the player and check the variables used to check for attachments
    (bind _isattachedoutput (Class|IControlAttach|IsAttachedOutput(Message) _returnvalue))
    (if _isattachedoutput
      (Class|IControlAttach|Attach(Message) (Game|Player|GetPlayerPawn 0) _self)
      (Class|IControlAttach|IsAttachedInput(Message) _returnvalue true))))

(event EventBeginPlay
  ;[1 1 1] Check if this specific actor, found using his display name, has a position saved. If he has he is moved to that location and than removed from the dict of actor saved
)

(fn ConstructionScript)

(fn IsAttachedOutput
  (return (Variables|Default|GetisAttached)))