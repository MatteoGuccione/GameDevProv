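; BP_Lever1 is a lever inventory item that restores its saved state when play begins.
; One tick after BeginPlay, it looks up its display name in the game instance's solved actors and hides itself without collision if found.
; Otherwise, if the saved inventory holds that name, it passes itself to the player pawn's inventory through GetItem.
; GetItemStruct exposes its Item data, while the other getters are empty interface stubs.
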(event EventBeginPlay
  (bind _self self)
  (bind _returnvalue (Utilities|GetDisplayName _self))
  (|CallParentFunction)
  (Utilities|FlowControl|DelayUntilNextTick)
  (bind _solvedactors (Class|IGet|GetSolvedActors(Message) (Game|GetGameInstance)))
  (if (Utilities|Array|ContainsItem _solvedactors _returnvalue)
    (Rendering|SetActorHiddenInGame true)
    (Collision|SetActorEnableCollision false)
    (else
      (bind _items (Class|IGet|GetItemsinInventory(Message) (Game|GetGameInstance)))
      (bind _array_element (Utilities|Array|ForEachLoopwithBreak _items :!label _label)
        (:LoopBody
          (if (Utilities|Enum|Equal(Enum) (.Name (Utilities|Struct|BreakS_ItemStructure _array_element)) (Utilities|Text|ToText(String) _returnvalue))
            (bind _inventory (Class|IGet|Getinventory(Message) (Game|Player|GetPlayerPawn 0)))
            (Default|GetItem _inventory self)
            (goto _label Break)))))))

(event Collision|EventActorBeginOverlap
  (params (OtherActor :type Actor%20Object%20Reference))
  (|CallParentFunction OtherActor) ; This node is disabled and will not be called.\nDrag off pins to build functionality.
)

(event EventTick
  (params (DeltaSeconds :type Float%20%28single-precision%29)))

(fn ConstructionScript
  (|CallParentFunction))

(fn GetActortoNotSpawn
  (return false))

(fn GetActorVelocity
  (return "0, 0, 0"))

(fn GetAttachedActor
  (return 0))

(fn GetAttachedActorLocal
  (return 0))

(fn GetAttachedActorName
  (return ""))

(fn GetAvailableJump
  (return 0))

(fn GetFirstStart
  (return false))

(fn Getinventory
  (return 0))

(fn GetIsAvailableforWallJump
  (return false))

(fn GetItemsinInventory
  (return 0))

(fn GetItemStruct
  (return (Variables|Default|GetItem)))

(fn GetKeys
  (return 0))

(fn GetNamePosition
  (return 0))

(fn GetPlayer&Actor
  (return 0))

(fn GetPlayerAbleTeleport
  (return false))

(fn GetPlayerForward
  (return "0, 0, 0"))

(fn GetSelfDialogueNumber
  (return 0))

(fn GetSolvedActorLocal
  (return 0))

(fn GetSolvedActors
  (return 0))

(fn GetSolvedPuzzle
  (return 0))