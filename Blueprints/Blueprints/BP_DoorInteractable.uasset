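; Interactable one-sided door that swings open when used from its correct side, optionally requiring a linked trigger object to be solved first.
; Interaction inside RightTrigger runs a Timeline yaw swing, then saves the door's name to the GameInstance's solved actors.
; Elsewhere, a FlipFlop toggles an "other side" dialogue and input lock.
; WrongTrigger's flag is unused, and BeginPlay's solved check leads nowhere.
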(event OnComponentBeginOverlap(RightTrigger)
  (params (OverlappedComponent :type Primitive%20Component%20Object%20Reference) (OtherActor :type Actor%20Object%20Reference) (OtherComp :type Primitive%20Component%20Object%20Reference) (OtherBodyIndex :type Integer) (bFromSweep :type Boolean) (SweepResult :type Hit%20Result%20Structure%20%28by%20ref%29))
  (if (Components|ComponentHasTag OtherComp "MainBody")
    (Variables|Default|SetisOverlappedGood true)))

(event OnComponentBeginOverlap(WrongTrigger)
  (params (OverlappedComponent :type Primitive%20Component%20Object%20Reference) (OtherActor :type Actor%20Object%20Reference) (OtherComp :type Primitive%20Component%20Object%20Reference) (OtherBodyIndex :type Integer) (bFromSweep :type Boolean) (SweepResult :type Hit%20Result%20Structure%20%28by%20ref%29))
  (if (Components|ComponentHasTag OtherComp "MainBody")
    (Variables|Default|SetisOverlappedWrong true)))

(event OnComponentEndOverlap(RightTrigger)
  (params (OverlappedComponent :type Primitive%20Component%20Object%20Reference) (OtherActor :type Actor%20Object%20Reference) (OtherComp :type Primitive%20Component%20Object%20Reference) (OtherBodyIndex :type Integer))
  (if (Components|ComponentHasTag OtherComp "MainBody")
    (Variables|Default|SetisOverlappedGood false)))

(event OnComponentEndOverlap(WrongTrigger)
  (params (OverlappedComponent :type Primitive%20Component%20Object%20Reference) (OtherActor :type Actor%20Object%20Reference) (OtherComp :type Primitive%20Component%20Object%20Reference) (OtherBodyIndex :type Integer))
  (if (Components|ComponentHasTag OtherComp "MainBody")
    (Variables|Default|SetisOverlappedWrong false)))

(event EventBeginPlay
  (|CallParentFunction)
  (bind _solvedactors (Class|IGet|GetSolvedActors(Message) (Game|GetGameInstance)))
  (if (Utilities|Array|ContainsItem _solvedactors (Utilities|GetDisplayName self))
    _))

(event EventSolved
  (Transformation|SetRelativeRotation (Variables|Default|GetDoor) (Math|Rotator|MakeRotator 0.0 0.0 1.8e+02) false false)
  (Development|PrintString "Hello"))

(event EventTick
  (params (DeltaSeconds :type Float%20%28single-precision%29))
  (|CallParentFunction DeltaSeconds) ; This node is disabled and will not be called.\nDrag off pins to build functionality.
)

(event EventInteraction
  (bind _returnvalue (Game|GetPlayerController 0))
  (bind _returnvalue_2 (Game|GetPlayerController 0))
  (bind _istriggerable (Variables|Default|GetisTriggerable))
  (bind _solvedactors (Class|IGet|GetSolvedActors(Message) (Game|GetGameInstance)))
  (if (and (Utilities|Array|ContainsItem _solvedactors (Utilities|GetDisplayName (Variables|Default|GetTriggeredObject))) _istriggerable)
    (if (Variables|Default|GetisOverlappedGood) :!label _label
      (Variables|Default|SetZRotation (.yaw (Variables|/Script/Engine.SceneComponent|GetRelativeRotation (Variables|Default|GetDoor))))
      (bind _doorfloat (Timeline|Timeline Play)
        (:Update
          (Variables|Default|SetdoorFloat _doorfloat)
          (Transformation|SetRelativeRotation (Variables|Default|GetDoor) (Math|Rotator|MakeRotator 0.0 0.0 (+ (Variables|Default|GetZRotation) (Math|Float|Lerp 0.0 1.2e+02 (Variables|Default|GetdoorFloat)))) false false))
        (:Finished
          (Class|ISave|SaveSolvedActor(Message) (Game|GetGameInstance) (Utilities|GetDisplayName self))))
      (else
        (Utilities|FlowControl|FlipFlop
          (:A
            (bind _returnvalue_3 (UserInterface|CreateWidget "/Game/Custom/Blueprints/Widgets/WB_Dialogue.WB_Dialogue_C" (Game|GetPlayerController 0)))
            (bind _output_get (Variables|Default|SetDialogueBox _returnvalue_3))
            (Variables|/Script/UMG.TextBlock|SetText (Variables|/Game/Custom/Blueprints/Widgets/WB_Dialogue.WB_Dialogue_C|GetDialogue1 _output_get) "Seems like it can be opened from the other side")
            (UserInterface|Viewport|AddtoViewport _output_get 0)
            (Input|SetIgnoreLookInput _returnvalue_2 true)
            (Input|SetIgnoreMoveInput _returnvalue_2 true)
            (Class|ISave|SaveinWidget(Message) _returnvalue_2 true))
          (:B
            (Widget|RemovefromParent (Variables|Default|GetDialogueBox))
            (Input|SetIgnoreLookInput _returnvalue false)
            (Input|SetIgnoreMoveInput _returnvalue false)
            (Class|ISave|SaveinWidget(Message) (Game|Player|GetPlayerPawn 0) false)))))
    (elif (not _istriggerable)
      (goto _label))))

(fn ConstructionScript
  (|CallParentFunction))