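; BP_KeyDemo is an interactable actor, apparently the demo's key, that brings up the demo end screen.
; Its Interaction event creates a WB_DemoEnd widget for player controller 0, adds it to the viewport and makes it visible.
; BeginPlay, overlap and Tick are disabled stubs, and the construction script only calls its parent.
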(event EventBeginPlay
  (|CallParentFunction) ; This node is disabled and will not be called.\nDrag off pins to build functionality.
)

(event Collision|EventActorBeginOverlap
  (params (OtherActor :type Actor%20Object%20Reference))
  (|CallParentFunction OtherActor) ; This node is disabled and will not be called.\nDrag off pins to build functionality.
)

(event EventTick
  (params (DeltaSeconds :type Float%20%28single-precision%29))
  (|CallParentFunction DeltaSeconds) ; This node is disabled and will not be called.\nDrag off pins to build functionality.
)

(event EventInteraction
  (bind _returnvalue (UserInterface|CreateWidget "/Game/Custom/Blueprints/Widgets/WB_DemoEnd.WB_DemoEnd_C" (Game|GetPlayerController 0)))
  (UserInterface|Viewport|AddtoViewport _returnvalue 0)
  (Widget|SetVisibility _returnvalue "Visible"))

(fn ConstructionScript
  (|CallParentFunction))